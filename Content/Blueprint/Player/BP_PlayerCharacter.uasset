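; BP_PlayerCharacter is the player character, with axis-driven movement and look, a weapon manager, and separate hands and body meshes.
; Input axes move it along the actor's forward and right vectors and turn the controller's pitch and yaw.
; On BeginPlay, only the authority has BPWeaponManager create and select a weapon.
; GetVisibleMash returns HandsMesh when locally controlled and the body Mesh otherwise.
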(event `InputAxis|MoveForward`
  (params (AxisValue :type "Float (single-precision)"))
  (`self.AddMovementInput` (`self.GetActorForwardVector`) AxisValue))

(event `InputAxis|LookUp`
  (params (AxisValue :type "Float (single-precision)"))
  (`self.AddControllerPitchInput` AxisValue))

(event `InputAxis|Turn`
  (params (AxisValue :type "Float (single-precision)"))
  (`self.AddControllerYawInput` AxisValue))

(event `InputAxis|MoveRight`
  (params (AxisValue :type "Float (single-precision)"))
  (`self.AddMovementInput` (`self.GetActorRightVector`) AxisValue))

(event `self.ReceiveBeginPlay`
  (`/Engine/EditorBlueprintResources/ActorMacros.Switch Has Authority`
    (:`Authority`
      (bind _weapon (`/Game/Blueprint/Component/Player/BP_WeaponManager.CreateWeapon` (`self.BP_WeaponManager`) null))
      (`/Game/Blueprint/Component/Player/BP_WeaponManager.SelectWeapon` (`self.BP_WeaponManager`) _weapon))))

(fn `GetVisibleMash`
  (returns (SkeletalMesh :type "SkeletalMeshComponent Object Reference"))
  (return (select `bool` (`self.IsLocallyControlled`) :`false` (`self.Mesh`) :`true` (`self.HandsMesh`))))

(fn `UserConstructionScript`)